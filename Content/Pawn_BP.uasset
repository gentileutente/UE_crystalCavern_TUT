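; Physics-driven rolling ball pawn that moves by forces and restarts the current level with a camera fade when damaged.
; Each Tick, macros move the spring arm over the sphere at its starting height, aim the camera at it, and apply input forces.
; Hit events mark it grounded, restoring force magnitudes and high damping; jumps push along the hit normal, then zero movement force and lower damping until the next hit.
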(event `self.ReceiveBeginPlay`
  (bind (_returnvalue_x _returnvalue_y _returnvalue_z) (`KismetMathLibrary.BreakVector` (`SceneComponent.K2_GetComponentLocation` (`self.Sphere`))))
  (set `self.initZ` _returnvalue_z)
  (`PlayerCameraManager.StartCameraFade` :`self` (`GameplayStatics.GetPlayerCameraManager` 0) :`FromAlpha` 1.0 :`Duration` 2.0))

(event `self.ReceiveTick`
  (params (DeltaSeconds :type "Float (single-precision)"))
  (bind (_movemagnitude_x _movemagnitude_y _movemagnitude_z) (`KismetMathLibrary.BreakVector` (`self.moveMagnitude`)))
  (bind (_movemagnitude_x_2 _movemagnitude_y_2) (`KismetMathLibrary.BreakVector` (`self.moveMagnitude`)))
  (bind (_returnvalue_x _returnvalue_y) (`KismetMathLibrary.BreakVector` (`SceneComponent.K2_GetComponentLocation` (`self.Sphere`))))
  (`SceneComponent.K2_SetWorldLocation` (`self.SpringArm`) (`KismetMathLibrary.MakeVector` _returnvalue_x _returnvalue_y (`self.initZ`)) false true)
  (`SceneComponent.K2_SetWorldRotation` (`self.Camera`) (`KismetMathLibrary.FindLookAtRotation` (`SceneComponent.K2_GetComponentLocation` (`self.Camera`)) (`SceneComponent.K2_GetComponentLocation` (`self.Sphere`))) false false)
  (`PrimitiveComponent.AddForce` (`self.Sphere`) (`KismetMathLibrary.MakeVector` (* (`self.GetInputAxisValue`) _movemagnitude_x_2) (* (`self.GetInputAxisValue`) _movemagnitude_y_2)) "None" true)
  (if (and (`self.doJump`) (`self.isGrounded`))
    (`PrimitiveComponent.AddForce` (`self.Sphere`) (* (`self.jumpVector`) _movemagnitude_z) "None" true)
    (set `self.doJump` false)
    (set `self.isGrounded` false)
    (set `self.moveMagnitude` (0.0 0.0 0.0))
    (`PrimitiveComponent.SetLinearDamping` (`self.Sphere`) 0.5)
    (else
      (set `self.doJump` false)
      (set `self.isGrounded` false))))

(event `InputAction|jump`
  (params (Key :type "Key Structure"))
  (:`Pressed`
    (set `self.doJump` true)))

(event `self.ReceiveHit`
  (params (MyComp :type "PrimitiveComponent Object Reference") (Other :type "Actor Object Reference") (OtherComp :type "PrimitiveComponent Object Reference") (bSelfMoved :type Boolean) (HitLocation :type "Vector Structure") (HitNormal :type "Vector Structure") (NormalImpulse :type "Vector Structure") (Hit :type "HitResult Structure (by ref)"))
  (set `self.isGrounded` true)
  (set `self.jumpVector` HitNormal)
  (set `self.moveMagnitude` (3000.0 3000.0 200000.0))
  (`PrimitiveComponent.SetLinearDamping` (`self.Sphere`) 5.0))

(event `Key|W`
  (params (Key :type "Key Structure"))
  (:`Pressed`
    (set `self.forwardPressed` true))
  (:`Released`
    (set `self.forwardPressed` false)))

(event `self.ReceiveAnyDamage`
  (params (Damage :type "Float (single-precision)") (DamageType :type "DamageType Object Reference") (InstigatedBy :type "Controller Object Reference") (DamageCauser :type "Actor Object Reference"))
  (`/Engine/EditorBlueprintResources/StandardMacros.DoOnce` false
    (:`Completed`
      (`PlayerCameraManager.StartCameraFade` :`self` (`GameplayStatics.GetPlayerCameraManager` 0) :`FromAlpha` 0.0 :`ToAlpha` 1.0 :`Duration` (`self.deathFadeTime`) :`bHoldWhenFinished` true)
      (bind _returnvalue (`GameplayStatics.GetCurrentLevelName` true))
      (`KismetSystemLibrary.Delay` (`self.deathFadeTime`))
      (`GameplayStatics.OpenLevel` (`KismetStringLibrary.Conv_StringToName` _returnvalue)))))

(fn `UserConstructionScript`)