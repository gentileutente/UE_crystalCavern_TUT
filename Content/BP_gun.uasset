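; An auto-firing cannon actor that repeatedly spawns projectiles at a fixed rate from BeginPlay.
; Each cycle waits for the Rate delay, spawns the Projectile class at the Arrow component's transform scaled by ProjScale, then plays a timeline.
; The timeline moves the barrel tip mesh along local Z, and its Start Fire event track loops back to the delay for the next shot.
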(event `self.ReceiveBeginPlay`
  (`KismetSystemLibrary.Delay` (`self.rate`) :!label _label)
  (`self.Fire`)
  (bind (_direction _barrell) (`Timeline|Timeline_0` :!via `PlayFromStart`)
    (:`Update`
      (`self.moveBarrell` _barrell))
    (:`startFire`
      (goto _label))))

(fn `Fire`
  (bind _arrow (`self.Arrow`))
  (`|SpawnActorFromClass` "/Game/projectile.projectile_C" (`KismetMathLibrary.MakeTransform` (`SceneComponent.K2_GetComponentLocation` _arrow) (`SceneComponent.K2_GetComponentRotation` _arrow) (`KismetMathLibrary.Conv_DoubleToVector` (`self.projScale`))) "Undefined" "OverrideRootScale" null null))

(fn `moveBarrell`
  (params (barrel_Z :type "Float (double-precision)"))
  (`SceneComponent.K2_SetRelativeLocation` (`self.cannonTipTest_001`) (`KismetMathLibrary.MakeVector` 0.0 0.0 barrel_Z) false false))

(fn `UserConstructionScript`)