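; Collectible crystal (gem) actor that flies into the player's ball on overlap, then destroys itself.
; A macro filters the overlap for the player, disables further overlap events on the collision component and stores the start location.
; A timeline then lerps the crystal toward the live position of the player's "ball"-tagged mesh.
; InitAbsorption duplicates the macro's setup but is not called in the event graph.
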(event `self.ReceiveActorBeginOverlap`
  (params (OtherActor :type "Actor Object Reference"))
  (`self.NewMacro_0` OtherActor)
  (bind (_direction _alpha_time) (`Timeline|TL_AbsorbeCrystal`)
    (:`Update`
      (`self.absorbAnimation` _alpha_time))
    (:`Finished`
      (`self.K2_DestroyActor`))))

(fn `absorbAnimation`
  (params (Alpha :type "Float (double-precision)"))
  (`self.K2_SetActorLocation` (`KismetMathLibrary.VLerp` (`self.lerp_start_vector`) (`SceneComponent.K2_GetComponentLocation` (`|GetArrayItem` (`self.GetComponentsByTag` (`GameplayStatics.GetPlayerPawn` 0) "/Script/Engine.StaticMeshComponent" "ball"))) Alpha)))

(fn `initAbsorption`
  (params (collidingActor :type "Object Object Reference"))
  (if (== collidingActor (`GameplayStatics.GetPlayerPawn` 0))
    (set `PrimitiveComponent.bGenerateOverlapEvents` false (`self.CollisionCMP`)) ; overalp only once!
    (set `self.lerp_start_vector` (`self.K2_GetActorLocation`)) ; read and set the start position of the GEM
  ))

(fn `UserConstructionScript`)